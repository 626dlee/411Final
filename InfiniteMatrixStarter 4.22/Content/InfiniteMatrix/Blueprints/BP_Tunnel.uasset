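; Tunnel segment for an endless obstacle run, with a spinning holed wall and two counter-rotating cave-rock pillars.
; Tick drives the rotation; the ±40 pillar checks compare a unit-vector component, so they never limit it.
; Trigger overlap spawns the next tunnel, destroys this one and counts passes for BP_Player; obstacle hits kill the player and reset the counter.
; RandomizeWall varies meshes and roll angles.
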(event OnComponentBeginOverlap(TriggerZone)
  (params (OverlappedComponent :type Primitive%20Component%20Object%20Reference) (OtherActor :type Actor%20Object%20Reference) (OtherComp :type Primitive%20Component%20Object%20Reference) (OtherBodyIndex :type Integer) (bFromSweep :type Boolean) (SweepResult :type Hit%20Result%20Structure%20%28by%20ref%29))
  (Default|SpawnTunnelatSpawnPoint (Variables|Components|GetTunnelSpawner))
  (Actor|DestroyActor)
  (Utilities|Casting|CastToBP_Player OtherActor)
  (Default|IncreaseWallsPassed (Variables|Default|GetGameManager)))

(event OnComponentHit(WallMesh)
  (params (HitComponent :type Primitive%20Component%20Object%20Reference) (OtherActor :type Actor%20Object%20Reference) (OtherComp :type Primitive%20Component%20Object%20Reference) (NormalImpulse :type Vector :default "0, 0, 0") (Hit :type Hit%20Result%20Structure%20%28by%20ref%29))
  (bind _asbp_player (Utilities|Casting|CastToBP_Player OtherActor))
  (Variables|/Game/InfiniteMatrix/Blueprints/BP_Player.BP_Player_C|SetisDead _asbp_player true)
  (Default|DisplayRestart _asbp_player)
  (Default|ResetCounter (Variables|Default|GetGameManager)))

(event OnComponentHit(Pillar2)
  (params (HitComponent :type Primitive%20Component%20Object%20Reference) (OtherActor :type Actor%20Object%20Reference) (OtherComp :type Primitive%20Component%20Object%20Reference) (NormalImpulse :type Vector :default "0, 0, 0") (Hit :type Hit%20Result%20Structure%20%28by%20ref%29))
  (bind _asbp_player (Utilities|Casting|CastToBP_Player OtherActor))
  (Variables|/Game/InfiniteMatrix/Blueprints/BP_Player.BP_Player_C|SetisDead _asbp_player true)
  (Default|DisplayRestart _asbp_player)
  (Default|ResetCounter (Variables|Default|GetGameManager)))

(event OnComponentHit(Pillar1)
  (params (HitComponent :type Primitive%20Component%20Object%20Reference) (OtherActor :type Actor%20Object%20Reference) (OtherComp :type Primitive%20Component%20Object%20Reference) (NormalImpulse :type Vector :default "0, 0, 0") (Hit :type Hit%20Result%20Structure%20%28by%20ref%29))
  (bind _asbp_player (Utilities|Casting|CastToBP_Player (stale OnComponentHit(Pillar2) OtherActor)))
  (Variables|/Game/InfiniteMatrix/Blueprints/BP_Player.BP_Player_C|SetisDead _asbp_player true)
  (Default|DisplayRestart _asbp_player)
  (Default|ResetCounter (Variables|Default|GetGameManager)))

(event EventBeginPlay)

(event EventTick
  (params (DeltaSeconds :type Float%20%28single-precision%29))
  (bind _returnvalue (Utilities|Time|GetWorldDeltaSeconds))
  (bind _rotatespeed (Variables|Components|GetRotateSpeed))
  (bind _pillar1 (Variables|Default|GetPillar1))
  (bind _pillar2 (Variables|Default|GetPillar2))
  (bind _returnvalue_2 (* _returnvalue _rotatespeed))
  (bind _returnvalue_3 (* _returnvalue_2 -1.0))
  (Transformation|AddLocalRotation (Variables|Default|GetWallMesh) (Math|Rotator|MakeRotator (* DeltaSeconds (Variables|Components|GetRotateSpeed)) 0.0 0.0) false false)
  (if (and (>= (.X (Math|Vector|BreakVector (Math|Rotator|GetRotationXVector (Transformation|GetWorldRotation (Variables|Default|GetPillar2))))) -4e+01) (<= (.X (Math|Vector|BreakVector (Math|Rotator|GetRotationXVector (Transformation|GetWorldRotation (Variables|Default|GetPillar2))))) 4e+01))
    (Transformation|AddLocalRotation (Variables|Default|GetPillar2) (Math|Rotator|MakeRotator _returnvalue_2 0.0 0.0) false false)
    (if (and (>= (.X (Math|Vector|BreakVector (Math|Rotator|GetRotationXVector (Transformation|GetWorldRotation (Variables|Default|GetPillar1))))) -4e+01) (<= (.X (Math|Vector|BreakVector (Math|Rotator|GetRotationXVector (Transformation|GetWorldRotation (Variables|Default|GetPillar1))))) 4e+01))
      (Transformation|AddLocalRotation (Variables|Default|GetPillar1) (Math|Rotator|MakeRotator _returnvalue_3 0.0 0.0) false false)
      (elif (>= (.X (Math|Vector|BreakVector (Math|Rotator|GetRotationXVector (Transformation|GetWorldRotation _pillar1)))) 4e+01)
        (Transformation|AddLocalRotation (Variables|Default|GetPillar1) (Math|Rotator|MakeRotator _returnvalue_3 0.0 0.0) false false)
        (elif (<= (.X (Math|Vector|BreakVector (Math|Rotator|GetRotationXVector (Transformation|GetWorldRotation _pillar1)))) -4e+01)
          (Transformation|AddLocalRotation (Variables|Default|GetPillar1) (Math|Rotator|MakeRotator (* _returnvalue_3 -1.0) 0.0 0.0) false false))))
    (elif (>= (.X (Math|Vector|BreakVector (Math|Rotator|GetRotationXVector (Transformation|GetWorldRotation _pillar2)))) 4e+01)
      (Transformation|AddLocalRotation (Variables|Default|GetPillar2) (Math|Rotator|MakeRotator 0.0 0.0 0.0) false false)
      (elif (<= (.X (Math|Vector|BreakVector (Math|Rotator|GetRotationXVector (Transformation|GetWorldRotation _pillar2)))) -4e+01)
        (Transformation|AddLocalRotation (Variables|Default|GetPillar2) (Math|Rotator|MakeRotator (* 0.0 -1.0) 0.0 0.0) false false)))))

(fn ConstructionScript)

(fn RandomizeWall
  (bind _wallmesh (Variables|Default|GetWallMesh))
  (Components|StaticMesh|SetStaticMesh (Variables|Default|GetPillar2) (Utilities|Select :Index (Math|Random|RandomIntegerinRange 0 3) :Option%200 "/Game/SoulCave/Environment/Meshes/Rocks/SM_Cave_Rocks_Stalactite_05.SM_Cave_Rocks_Stalactite_05" :Option%201 "/Game/SoulCave/Environment/Meshes/Rocks/SM_Cave_Rocks_Stalactite_04.SM_Cave_Rocks_Stalactite_04" :Option%202 "/Game/SoulCave/Environment/Meshes/Rocks/SM_Cave_Rocks_Stalactite_02.SM_Cave_Rocks_Stalactite_02" :Option%203 "/Game/SoulCave/Environment/Meshes/Building/SM_Cave_Rock_Pillar01REDO.SM_Cave_Rock_Pillar01REDO"))
  (Transformation|AddLocalRotation (Variables|Default|GetPillar2) (Math|Rotator|MakeRotator (Math|Random|RandomFloatinRange -4e+01 4e+01) 0.0 0.0) false false)
  (Components|StaticMesh|SetStaticMesh (Variables|Default|GetPillar1) (Utilities|Select :Index (Math|Random|RandomIntegerinRange 0 3) :Option%200 "/Game/SoulCave/Environment/Meshes/Rocks/SM_Cave_Rocks_Stalactite_05.SM_Cave_Rocks_Stalactite_05" :Option%201 "/Game/SoulCave/Environment/Meshes/Rocks/SM_Cave_Rocks_Stalactite_04.SM_Cave_Rocks_Stalactite_04" :Option%202 "/Game/SoulCave/Environment/Meshes/Rocks/SM_Cave_Rocks_Stalactite_02.SM_Cave_Rocks_Stalactite_02" :Option%203 "/Game/SoulCave/Environment/Meshes/Building/SM_Cave_Rock_Pillar01REDO.SM_Cave_Rock_Pillar01REDO"))
  (Transformation|AddLocalRotation (Variables|Default|GetPillar1) (Math|Rotator|MakeRotator (Math|Random|RandomFloatinRange -4e+01 4e+01) 0.0 0.0) false false)
  (Components|StaticMesh|SetStaticMesh _wallmesh (Utilities|Select :Index (Math|Random|RandomIntegerinRange 0 3) :Option%200 "/Game/InfiniteMatrix/Meshes/SM_Hole_01.SM_Hole_01" :Option%201 "/Game/InfiniteMatrix/Meshes/SM_Hole_02.SM_Hole_02" :Option%202 "/Game/InfiniteMatrix/Meshes/SM_Hole_03.SM_Hole_03" :Option%203 "/Game/InfiniteMatrix/Meshes/SM_Hole_04.SM_Hole_04"))
  (Transformation|AddLocalRotation _wallmesh (Math|Rotator|MakeRotator (Math|Random|RandomFloatinRange 0.0 3.6e+02) 0.0 0.0) false false))