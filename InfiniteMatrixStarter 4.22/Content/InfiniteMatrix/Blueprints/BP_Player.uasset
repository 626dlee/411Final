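; Player pawn for an endless forward-moving game, steered by touch drag or up/right input axes using swept local offsets.
; While alive, Tick pushes it forward and keeps raising ForwardSpeed, multiplicatively at first, then linearly past a threshold.
; ChangeForwardSpeed adds a fixed speed step when called.
; DisplayRestart shows the score in the restart widget with UI-only input, and RestartGame clears it, resetting speed, death flag and GameManager's wall count.
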(event EventTick
  (params (DeltaSeconds :type Float%20%28single-precision%29))
  (bind _returnvalue (Game|GetPlayerController 0))
  (bind (_locationx _locationy _biscurrentlypressed) (Class|PlayerController|GetInputTouchState _returnvalue "Touch1"))
  (if (not (Variables|Default|GetisDead))
    (if _biscurrentlypressed
      (Variables|Default|SetNewTouch (Math|Vector2D|MakeVector2D _locationx _locationy))
      (Transformation|AddActorLocalOffset (Math|Vector|MakeVector (* DeltaSeconds (Variables|Default|GetForwardSpeed)) (* 5.0 (.X (Math|Vector2D|BreakVector2D (- (Variables|Default|GetNewTouch) (Variables|Default|GetLastTouch))))) (* 5.0 (* (.Y (Math|Vector2D|BreakVector2D (- (Variables|Default|GetNewTouch) (Variables|Default|GetLastTouch)))) -1.0))) true false)
      (Variables|Default|SetLastTouch (Variables|Default|GetNewTouch))
      (if (<= (* (Variables|Default|GetForwardSpeed) 1.001) 5e+03)
        (Variables|Default|SetForwardSpeed (* (Variables|Default|GetForwardSpeed) 1.001))
        (else
          (Variables|Default|SetForwardSpeed (+ (Variables|Default|GetForwardSpeed) 1.0))))
      (else
        (Transformation|AddActorLocalOffset (Math|Vector|MakeVector (* DeltaSeconds (Variables|Default|GetForwardSpeed)) 0.0 0.0) true false)
        (if (<= (stale _output_get) 5e+03)
          (bind _output_get (Variables|Default|SetForwardSpeed (* (Variables|Default|GetForwardSpeed) 1.001)))
          (else
            (Variables|Default|SetForwardSpeed (+ (Variables|Default|GetForwardSpeed) 1.0))))))))

(event EventBeginPlay
  (bind _returnvalue (UserInterface|CreateWidget "/Game/InfiniteMatrix/UI/WBP_Restart.WBP_Restart_C"))
  (Variables|Default|SetrestartWidget _returnvalue))

(event Input|AxisEvents|InputAxisMoveUp
  (params (AxisValue :type Float%20%28single-precision%29))
  ;[1 1 1] Horizontal and vertical movement
  (Pawn|Input|AddMovementInput (Transformation|GetActorUpVector) (* AxisValue (Variables|Default|GetMoveSpeed) 3.5) false)
  (bind _returnvalue (Class|Pawn|ConsumeMovementInputVector))
  (Transformation|AddActorLocalOffset (* _returnvalue (Utilities|Time|GetWorldDeltaSeconds)) true false))

(event Input|AxisEvents|InputAxisMoveRight
  (params (AxisValue :type Float%20%28single-precision%29))
  ;[1 1 1] Horizontal and vertical movement
  (Pawn|Input|AddMovementInput (Transformation|GetActorRightVector) (* AxisValue (Variables|Default|GetMoveSpeed) 3.5) false)
  (bind _returnvalue (Class|Pawn|ConsumeMovementInputVector))
  (Transformation|AddActorLocalOffset (* _returnvalue (Utilities|Time|GetWorldDeltaSeconds)) true false))

(event Input|TouchEvents|Touch1
  (params (Key :type Key%20Structure))
  (bind _returnvalue (Game|GetPlayerController 0))
  (bind (_locationx _locationy) (Class|PlayerController|GetInputTouchState _returnvalue "Touch1"))
  (:Pressed
    (Variables|Default|SetLastTouch (Math|Vector2D|MakeVector2D _locationx _locationy))))

(fn ConstructionScript)

(fn DisplayRestart
  (bind _returnvalue (Game|GetPlayerController 0))
  (bind _restartwidget (Variables|Default|GetrestartWidget))
  (Default|UpdateScoreText _restartwidget (Math|Conversions|ToInteger(Byte) (Utilities|GetDisplayName (Variables|/Game/InfiniteMatrix/UI/WBP_HUD.WBP_HUD_C|GetCounterText (Variables|Default|Gethudwidget)))))
  (UserInterface|Viewport|AddtoViewport _restartwidget 0)
  (Input|SetInputModeUIOnly _returnvalue 0 "DoNotLock")
  (Variables|/Script/Engine.PlayerController|SetbShowMouseCursor _returnvalue true))

(fn RestartGame
  (bind _returnvalue (Game|GetPlayerController 0))
  (Variables|Default|SetisDead false)
  (bind _foundwidgets (Widget|GetAllWidgetsOfClass "/Game/InfiniteMatrix/UI/WBP_Restart.WBP_Restart_C" false))
  (Utilities|FlowControl|Sequence
    (:then_0
      (for _array_element _foundwidgets
        (Widget|RemovefromParent _array_element)))
    (:then_1
      (Variables|Default|SetForwardSpeed 8.5e+02)
      (Input|SetInputModeGameOnly _returnvalue)
      (Variables|/Script/Engine.PlayerController|SetbShowMouseCursor _returnvalue false))
    (:then_2
      (Development|PrintString "restartGameCalled")
      (Variables|/Game/InfiniteMatrix/Blueprints/BP_GameManager.BP_GameManager_C|SetWallsPassed (Variables|Default|GetGameManager) 0))))

(fn ChangeForwardSpeed
  (if (not (== (Variables|Default|GetForwardSpeed) 2.5e+03))
    (Variables|Default|SetForwardSpeed (+ (Variables|Default|GetForwardSpeed) 25.0))
    (Development|PrintString "Forward Speed Changed")))